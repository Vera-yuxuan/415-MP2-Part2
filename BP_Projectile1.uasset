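; BP_Projectile1 is a projectile that deals damage on sphere overlap, with BP_Mortar1 exempt.
; Overlapping the learning-kit player character or a House applies damage, spawns a Niagara burst and destroys the projectile.
; Other overlaps spawn the burst, then apply reduced damage and destroy the projectile only if the player is within a short radius, so distant impacts leave it alive.
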(event `self.Sphere.OnComponentBeginOverlap`
  (params (OverlappedComponent :type "PrimitiveComponent Object Reference") (OtherActor :type "Actor Object Reference") (OtherComp :type "PrimitiveComponent Object Reference") (OtherBodyIndex :type Integer) (bFromSweep :type Boolean) (SweepResult :type "HitResult Structure (by ref)"))
  (bind _returnvalue (`self.K2_GetActorLocation`))
  (bind _asbp_learning_kit_player_character (cast `/Game/LearningKit_Games/Blueprints/PlayerCharacter/BP_LearningKit_PlayerCharacter` OtherActor)
    (:`then`
      (`GameplayStatics.ApplyDamage` _asbp_learning_kit_player_character 20.0 null self)
      (`NiagaraFunctionLibrary.SpawnSystemAtLocation` "/Game/LearningKit_Robots/VFX/Bursts/NS_Burst_Simple.NS_Burst_Simple" (`self.K2_GetActorLocation`))
      (`self.K2_DestroyActor` :!label _label))
    (:`CastFailed`
      (bind _ashouse (cast `/Game/LearningKit_Games/Blueprints/Enemies/House` OtherActor)
        (:`then`
          (`GameplayStatics.ApplyDamage` _ashouse 20.0 null self)
          (`NiagaraFunctionLibrary.SpawnSystemAtLocation` "/Game/LearningKit_Robots/VFX/Bursts/NS_Burst_Simple.NS_Burst_Simple" (`self.K2_GetActorLocation`))
          (goto _label))
        (:`CastFailed`
          (cast `/Game/LearningKit_Games/Blueprints/Enemies/BP_Mortar1` OtherActor
            (:`CastFailed`
              (`NiagaraFunctionLibrary.SpawnSystemAtLocation` "/Game/LearningKit_Robots/VFX/Bursts/NS_Burst_Simple.NS_Burst_Simple" _returnvalue)
              (if (<= (`KismetMathLibrary.Vector_Distance` (`self.K2_GetActorLocation` (`GameplayStatics.GetPlayerCharacter` 0)) _returnvalue) 300.0)
                (`GameplayStatics.ApplyDamage` (`GameplayStatics.GetPlayerCharacter` 0) 10.0 null self)
                (goto _label)))))))))

(fn `UserConstructionScript`)
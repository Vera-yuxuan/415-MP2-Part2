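; BP_Pursuer is an AI enemy that chases the player, dealing damage on arrival, and destroys itself when the player overlaps its Box.
; It chases from BeginPlay, repeating after each successful hit and short delay.
; AIPerception updates choose chasing or self-looping random roaming by player distance.
; Roaming centers on SpawnLocation, but that variable's assignment and an AIState switch are unwired.
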(event `self.ReceiveBeginPlay`
  (`self.ChasePlayer`))

(event `self.ReceiveTick`
  (params (DeltaSeconds :type "Float (single-precision)")))

(event `Roam`
  (`|AIMoveTo` self (`NavigationSystemV1.K2_GetRandomReachablePointInRadius` (`self.SpawnLocation`) 750.0 null null) null
    (:`then`
      (`KismetSystemLibrary.Delay` 5.0)
      (`self.Roam`))))

(event `ChasePlayer`
  (`|AIMoveTo` self (0.0 0.0 0.0) (`GameplayStatics.GetPlayerCharacter` 0)
    (:`OnSuccess`
      (`GameplayStatics.ApplyDamage` (`GameplayStatics.GetPlayerCharacter` 0) 15.0 null self)
      (`GameplayStatics.PlaySoundAtLocation` "/Game/LearningKit_Robots/Audio/Goal_Cue.Goal_Cue" (`self.K2_GetActorLocation` self) (struct) 1.0 1.0 0.0 null null null null)
      (`KismetSystemLibrary.Delay` 2.0)
      (`self.ChasePlayer`))))

(event `self.AIPerception.OnPerceptionUpdated`
  (params (UpdatedActors :type "Array of Actor Object Reference (by ref)"))
  (for _array_element UpdatedActors
    (bind _asbp_learning_kit_player_character (cast `/Game/LearningKit_Games/Blueprints/PlayerCharacter/BP_LearningKit_PlayerCharacter` _array_element))
    (if (<= (`KismetMathLibrary.Vector_Distance` (`self.K2_GetActorLocation` _asbp_learning_kit_player_character) (`self.K2_GetActorLocation` self)) 800.0)
      (`self.ChasePlayer`)
      (else
        (`self.Roam`)))))

(event `self.Box.OnComponentBeginOverlap`
  (params (OverlappedComponent :type "PrimitiveComponent Object Reference") (OtherActor :type "Actor Object Reference") (OtherComp :type "PrimitiveComponent Object Reference") (OtherBodyIndex :type Integer) (bFromSweep :type Boolean) (SweepResult :type "HitResult Structure (by ref)"))
  (cast `/Game/LearningKit_Games/Blueprints/PlayerCharacter/BP_LearningKit_PlayerCharacter` OtherActor)
  (`self.K2_DestroyActor`))

(fn `UserConstructionScript`)